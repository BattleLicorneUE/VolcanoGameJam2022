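; BP_GameManager watches map progression and declares a win when enough zones are complete.
; BeginPlay starts a looping timer several times a second, presumably driving CheckMapProgression, which counts valid AllZones entries with a "Complete" status.
; When the count reaches the array's last index, one short of its length, it prints a win message.
; A DoOnce resets after each unsuccessful check, so the win fires only once.
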(event Custom|CheckMapProgression
  (bind _allzones (Variables|Default|GetAllZones))
  (Utilities|FlowControl|DoOnce false :!label _label
    (:Completed
      (Variables|Default|SetCompleteZoneNB 0)
      (bind _array_element (Utilities|Array|ForEachLoopwithBreak _allzones)
        (:LoopBody
          (Utilities|IsValid _array_element
            (:Is%20Valid
              (if (Utilities|Enum|Equal(Enum) (Variables|/Game/Blueprints/ZoneRepartition/BP_ZoneManager.BP_ZoneManager_C|GetZoneStatus _array_element) (Utilities|Text|MakeLiteralText "Complete"))
                (Math|Integer|IncrementInt (Variables|Default|GetCompleteZoneNB))))))
        (:Completed
          (if (>= (Variables|Default|GetCompleteZoneNB) (Utilities|Array|LastIndex _allzones))
            (Development|PrintString "YOU WIN!!")
            (else
              (goto _label Reset))))))))

(event EventBeginPlay
  (Utilities|Time|SetTimerbyEvent (EventDispatchers|CreateEvent :!event Custom|CheckMapProgression) 0.333333 true))

(event Collision|EventActorBeginOverlap
  (params (OtherActor :type Actor%20Object%20Reference)))

(event EventTick
  (params (DeltaSeconds :type Float%20%28single-precision%29)))

(fn ConstructionScript)