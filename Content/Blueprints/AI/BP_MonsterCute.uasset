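; BP_MonsterCute is a monster Blueprint that shows its remaining health by swapping the material on its sphere.
; Incoming damage is subtracted from current health, then a server event relays the new value to a multicast event.
; The multicast calls UpdateColorHealth, which picks one of three materials by health threshold.
; No death handling is present, so zero health keeps the lowest-tier material.
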(event Custom|Multicast%20Update%20Color%20Health
  (params (Health :type Float%20%28double-precision%29) (Target :type Primitive%20Component%20Object%20Reference))
  (CallFunction|UpdateColorHealth Health Target))

(event Custom|Server%20Update%20Color%20Health
  (params (Health :type Float%20%28double-precision%29) (Target :type Primitive%20Component%20Object%20Reference))
  (CallFunction|MulticastUpdateColorHealth Health Target))

(event Game|Damage|EventAnyDamage
  (params (Damage :type Float%20%28single-precision%29) (DamageType :type Damage%20Type%20Object%20Reference) (InstigatedBy :type Controller%20Object%20Reference) (DamageCauser :type Actor%20Object%20Reference))
  (Variables|Default|SetHealth_Current (- (Variables|Default|GetHealth_Current) Damage))
  (CallFunction|ServerUpdateColorHealth (Variables|Default|GetHealth_Current) (Variables|Default|GetSphere)))

(fn ConstructionScript)

(fn UpdateColorHealth
  (params (Health :type Float%20%28double-precision%29) (Target :type Primitive%20Component%20Object%20Reference))
  (if (>= Health 6e+01)
    (Rendering|Material|SetMaterial Target 0 (Variables|Default|GetMaterial))
    (elif (>= Health 4e+01)
      (Rendering|Material|SetMaterial Target 0 (Variables|Default|GetMaterial_0))
      (else
        (if (>= Health 1.0)
          _
          (else
            _))
        (Rendering|Material|SetMaterial Target 0 (Variables|Default|GetMaterial_1))))))