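; AI controller for BP_MonsterCute that starts and feeds its behavior tree.
; On possess it caches the monster, waits briefly, runs BT_MonsterCute_BehaviorTree, then writes the monster's character reference to the RefCharacterPawn blackboard key and sets an initial state.
; UpdateBehaviorMonsterCute stores the behavior state and mirrors it to the State_MonsterCute blackboard enum key.
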(event EventPossess
  (params (PossessedPawn :type Pawn%20Object%20Reference))
  (bind _asbp_monster_cute (Utilities|Casting|CastToBP_MonsterCute PossessedPawn))
  (Variables|Default|SetAs%20BP%20Monster%20Cute _asbp_monster_cute)
  (Utilities|FlowControl|Delay 1.0)
  (bind _returnvalue (AI|RunBehaviorTree "/Game/Blueprints/AI/BT_MonsterCute_BehaviorTree.BT_MonsterCute_BehaviorTree"))
  (if _returnvalue
    (AI|Components|Blackboard|SetValueasObject (AI|GetBlackboard 0) (Utilities|Name|MakeLiteralName "RefCharacterPawn") (Variables|/Game/Blueprints/AI/BP_MonsterCute.BP_MonsterCute_C|Getref%20My%20Character (Variables|Default|GetAs%20BP%20Monster%20Cute)))
    (CallFunction|UpdateBehaviorMonsterCute "NewEnumerator0")))

(fn ConstructionScript)

(fn UpdateBehaviorMonsterCute
  (params (State%20Behavior :type E_State_MonsterCute%20Enum :default "NewEnumerator0"))
  (bind _output_get (Variables|Default|SetState%20Behavior State%20Behavior))
  (AI|Components|Blackboard|SetValueasEnum (AI|GetBlackboard 0) (Utilities|Name|MakeLiteralName "State_MonsterCute") _output_get))