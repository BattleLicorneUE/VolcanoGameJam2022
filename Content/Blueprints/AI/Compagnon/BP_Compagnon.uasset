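; BP_Compagnon is a companion pet that the player feeds from their inventory to restore its health and calories.
; Looping timers and check events handle calorie text and light damage when the player's air value drops below carbon.
; Damage lowers health and swaps the mesh material by threshold through a server-to-multicast event chain.
; Overlap toggles a "Feed Pet" prompt and calorie display, and a separate event sets widget dialogue.
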(event Custom|Multicast%20Update%20Color%20Health
  (params (Health :type Float%20%28double-precision%29) (Target :type Primitive%20Component%20Object%20Reference))
  (CallFunction|UpdateColorHealth Health Target))

(event Custom|Server%20Update%20Color%20Health
  (params (Health :type Float%20%28double-precision%29) (Target :type Primitive%20Component%20Object%20Reference))
  (CallFunction|MulticastUpdateColorHealth Health Target))

(event Custom|CheckAirQuality
  (bind _asbp_character_master (Utilities|Casting|CastToBP_Character_Master (Game|GetPlayerCharacter 0)))
  (if (< (.AirValue (Utilities|Struct|BreakStruct_Save (Variables|/Game/Blueprints/BP_Character_Master.BP_Character_Master_C|GetSaveInfo _asbp_character_master))) (.CarbonValue (Utilities|Struct|BreakStruct_Save (Variables|/Game/Blueprints/BP_Character_Master.BP_Character_Master_C|GetSaveInfo _asbp_character_master))))
    (Game|Damage|ApplyDamage self 0.1 0 0)))

(event Custom|CheckCalorieAmount
  (Rendering|Components|TextRender|SetText (Variables|Default|GetCalorieAmount) (Utilities|Text|ToText(Float) (Variables|Default|GetCurrentCalorie) "HalfToEven")))

(event Custom|Update%20Widget%20Dialogue
  (params (Dialogue :type Text))
  (bind _asbp_widget_dialogue (Utilities|Casting|CastToBP_WidgetDialogue (UserInterface|GetUserWidgetObject (Variables|Default|GetWidget))))
  (Variables|/Game/Blueprints/Constructions/Widgets/BP_WidgetDialogue.BP_WidgetDialogue_C|SetDialogue _asbp_widget_dialogue Dialogue))

(event Game|Damage|EventAnyDamage
  (params (Damage :type Float%20%28single-precision%29) (DamageType :type Damage%20Type%20Object%20Reference) (InstigatedBy :type Controller%20Object%20Reference) (DamageCauser :type Actor%20Object%20Reference))
  (Variables|Default|SetHealth_Current (- (Variables|Default|GetHealth_Current) Damage))
  (CallFunction|ServerUpdateColorHealth (Variables|Default|GetHealth_Current) (Variables|Default|GetStaticMesh)))

(event EventBeginPlay
  (Utilities|Time|SetTimerbyEvent (EventDispatchers|CreateEvent :!event Custom|CheckAirQuality) 0.333333 true)
  (Utilities|Time|SetTimerbyEvent (EventDispatchers|CreateEvent :!event Custom|CheckCalorieAmount) 0.333333 true))

(event EventOnInteract
  (bind _asbp_character_master (Utilities|Casting|CastToBP_Character_Master (Game|GetPlayerCharacter 0)))
  (Default|RemoveFoodfromInventory _asbp_character_master)
  (Variables|Default|SetHealth_Current (Math|Float|Clamp(Float) (+ (Variables|Default|GetHealth_Current) 15.0) 0.0 (Variables|Default|GetHealth_Max)))
  (Variables|Default|SetCurrentCalorie (Math|Float|Clamp(Float) (+ (Variables|Default|GetCurrentCalorie) 15.0) 0.0 (Variables|Default|GetMaxCalorie))))

(event EventOnExitOverlap
  (Widget|RemovefromParent (stale EventOnOverlap _returnvalue))
  (Rendering|SetVisibility (Variables|Default|GetCalorieAmount) false false))

(event EventOnOverlap
  (bind _returnvalue (UserInterface|CreateWidget "/Game/Interfaces/InteractInterfaces/W_InteractMessage.W_InteractMessage_C" 0 "Feed Pet"))
  (UserInterface|Viewport|AddtoViewport _returnvalue 0)
  (Rendering|SetVisibility (Variables|Default|GetCalorieAmount) true false))

(fn ConstructionScript)

(fn UpdateColorHealth
  (params (Health :type Float%20%28double-precision%29) (Target :type Primitive%20Component%20Object%20Reference))
  (if (>= Health 6e+01)
    (Rendering|Material|SetMaterial Target 0 (Variables|Default|GetMaterial))
    (elif (>= Health 4e+01)
      (Rendering|Material|SetMaterial Target 0 (Variables|Default|GetMaterial_0))
      (else
        (if (>= Health 1.0)
          _
          (else
            _))
        (Rendering|Material|SetMaterial Target 0 (Variables|Default|GetMaterial_1))))))