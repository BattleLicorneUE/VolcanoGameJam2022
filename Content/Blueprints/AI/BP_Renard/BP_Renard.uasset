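; BP_Renard is an AI fox that wanders around its spawn point and can affect the player's carbon and air values.
; From BeginPlay it moves to random reachable points within a radius of its origin, pausing a random few seconds after each success or failure before repeating.
; Its UpdateImpact event adds its Value to the player character's carbon and removes the same amount from air.
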(event Custom|MoveRandom
  (AI|AIMoveTo self (.RandomLocation (AI|Navigation|GetRandomReachablePointinRadius (Variables|Default|GetPositionOrigin) 5e+02 0 0)) 0 5.0 false
    (:OnSuccess
      _)
    (:OnFail
      _))
  (Utilities|FlowControl|Delay (Math|Random|RandomFloatinRange 2.0 1e+01))
  (CallFunction|MoveRandom))

(event EventBeginPlay
  (Variables|Default|SetPositionOrigin (Transformation|GetActorLocation))
  (CallFunction|MoveRandom))

(event EventUpdateImpact
  (bind _value (Variables|Default|GetValue))
  (bind _asbp_character_master (Utilities|Casting|CastToBP_Character_Master (Game|GetPlayerCharacter 0)))
  (Default|AddCarbonValue _asbp_character_master _value)
  (Default|RemoveAirValue _asbp_character_master _value))

(fn ConstructionScript)