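; Interactable pet selection point that lets the player acquire a Water, Earth or Fire companion.
; Overlap shows an interact message widget naming the pet, removed when the overlap ends.
; On interact, it switches on PetName and has the player's BP_Character_Master spawn the matching companion at the character mesh's location.
; It then destroys the pet model, every actor in ActorsToDisable and itself.
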(event EventBeginPlay)

(event Collision|EventActorBeginOverlap
  (params (OtherActor :type Actor%20Object%20Reference)))

(event EventTick
  (params (DeltaSeconds :type Float%20%28single-precision%29)))

(event EventOnInteract
  (bind _returnvalue (Game|GetPlayerCharacter 0))
  (bind _mesh (Variables|/Script/Engine.Character|GetMesh _returnvalue))
  (bind _returnvalue_2 (Transformation|GetWorldLocation _mesh))
  (Development|PrintString (Utilities|String|Append "you acquired " (Utilities|String|ToString(Byte) (Variables|Default|GetPetName))))
  (switch Utilities|FlowControl|Switch|SwitchonE_Companiontypes (Variables|Default|GetPetName)
    (:NewEnumerator0
      (bind _asbp_character_master (Utilities|Casting|CastToBP_Character_Master _returnvalue))
      (Default|SpawnCompanion _asbp_character_master "/Game/Blueprints/AI/Compagnon/BP_Compagnon_Water.BP_Compagnon_Water_C" _returnvalue_2))
    (:NewEnumerator1
      (bind _asbp_character_master_2 (Utilities|Casting|CastToBP_Character_Master _returnvalue))
      (Default|SpawnCompanion _asbp_character_master_2 "/Game/Blueprints/AI/Compagnon/BP_Compagnon_Earth.BP_Compagnon_Earth_C" _returnvalue_2))
    (:NewEnumerator2
      (bind _asbp_character_master_3 (Utilities|Casting|CastToBP_Character_Master _returnvalue))
      (Default|SpawnCompanion _asbp_character_master_3 "/Game/Blueprints/AI/Compagnon/BP_Compagnon_Fire.BP_Compagnon_Fire_C" _returnvalue_2)))
  (Actor|DestroyActor (Variables|Default|Getpetmodel))
  (for _array_element (Variables|Default|GetActorsToDisable)
    (Actor|DestroyActor _array_element))
  (Actor|DestroyActor))

(event EventOnExitOverlap
  (Widget|RemovefromParent (stale EventOnOverlap _returnvalue)))

(event EventOnOverlap
  (bind _returnvalue (UserInterface|CreateWidget "/Game/Interfaces/InteractInterfaces/W_InteractMessage.W_InteractMessage_C" 0 (Utilities|Text|FormatText "select {petname}" (Utilities|Select :Index (Variables|Default|GetPetName) :NewEnumerator0 "Water pet" :NewEnumerator1 "Earth pet" :NewEnumerator2 "Fire pet"))))
  (UserInterface|Viewport|AddtoViewport _returnvalue 0))

(fn ConstructionScript)