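; BP_PlayerController is the player controller that handles camera look, mouse cursor toggling and avatar swapping for the player's BP_Character_Master pawn.
; On BeginPlay it caches the controlled character, then forwards IA_Look input to its CameraInput while CanTurn is true.
; Holding IA_ShowMouse shows the cursor and blocks turning.
; ChangeAvatarByID sets the character's skeletal mesh from AvatarList by index, applies the shared master AnimBlueprint and records the ID.
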(event Input|EnhancedActionEvents|EnhancedInputActionIA_Look
  (params (ActionValue :type Vector%202D%20Structure) (ElapsedSeconds :type Float%20%28double-precision%29) (TriggeredSeconds :type Float%20%28double-precision%29) (InputAction :type Input%20Action%20Object%20Reference :default "/Game/ThirdPerson/Input/Actions/IA_Look.IA_Look"))
  ;[1 1 1] Camera Look Input
  (:Triggered
    (if (Variables|Default|GetCanTurn?)
      (Default|CameraInput (Variables|Default|GetAs%20BP%20Character%20Master) (.x ActionValue) (.y ActionValue)))))

(event Input|EnhancedActionEvents|EnhancedInputActionIA_ShowMouse
  (params (ActionValue :type Boolean) (ElapsedSeconds :type Float%20%28double-precision%29) (TriggeredSeconds :type Float%20%28double-precision%29) (InputAction :type Input%20Action%20Object%20Reference :default "/Game/ThirdPerson/Input/Actions/IA_ShowMouse.IA_ShowMouse"))
  ;[1 1 1] ShowMouse input
  (:Started
    (Variables|Default|SetbShowMouseCursor true)
    (Variables|Default|SetCanTurn? false))
  (:Completed
    (Variables|Default|SetbShowMouseCursor false)
    (Variables|Default|SetCanTurn? true)))

(event EventBeginPlay
  ;[1 1 1] BEGINPLAY
  ;[1 1 1] SEQUENCE
  (Utilities|FlowControl|Sequence
    (:then_0
      ;[1 1 1] REF TO CHARACTER
      (bind _asbp_character_master (Utilities|Casting|CastToBP_Character_Master (Pawn|GetControlledPawn)))
      (Variables|Default|SetAs%20BP%20Character%20Master _asbp_character_master))))

(fn ConstructionScript)

(fn ChangeAvatarbyID
  (params (ID :type Integer))
  (bind _as_bp_character_master (Variables|Default|GetAs%20BP%20Character%20Master))
  (bind _mesh (Variables|/Script/Engine.Character|GetMesh _as_bp_character_master))
  (Components|SkeletalMesh|SetSkeletalMeshAsset _mesh (Utilities|Array|Get(acopy) (Variables|Default|GetAvatarList) ID))
  (Class|SkeletalMeshComponent|SetAnimClass _mesh "/Game/Characters/BattleLicorne/Master_Skeleton_AnimBlueprint.Master_Skeleton_AnimBlueprint_C")
  (Variables|Default|SetCurrentAvatarID ID))