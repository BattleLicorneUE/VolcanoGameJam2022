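; Game instance Blueprint that hosts and joins multiplayer sessions through Advanced Sessions nodes.
; CreateSession creates a session, then opens the GameplayAbility level as a listen server on success.
; SearchSession finds sessions on all server types and attempts to join every result in a loop, without filtering or stopping at the first.
; Each step, plus any travel error, reports through on-screen debug prints.
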(event Custom|Create%20Session
  (params (PlayerController :type Player%20Controller%20Object%20Reference))
  (|AdvancedSession 0 PlayerController 100 0 false true false true true true false false false true false true
    (:then
      (Development|PrintString "Try Connected"))
    (:OnSuccess
      (Game|OpenLevel(byName) "GameplayAbility" true "listen")
      (Development|PrintString "OnSuccessConnected"))
    (:OnFailure
      (Development|PrintString "OnFailureConnected"))))

(event Custom|Search%20Session
  (params (PlayerController :type Player%20Controller%20Object%20Reference))
  (bind _results (|FindSessionsAdvanced PlayerController 100 false "AllServers" 0 false false false true)
    (:then
      (Development|PrintString "Try Find"))
    (:OnSuccess
      (for _array_element _results
        (|JoinSession PlayerController _array_element
          (:then
            (Development|PrintString "Try join"))
          (:OnSuccess
            (Development|PrintString "Join On Success"))
          (:OnFailure
            (Development|PrintString "Join On Failure"))))
      (Development|PrintString (Utilities|String|Append "Session found : " (Utilities|String|ToString(Integer) (Utilities|Array|Length _results)))))
    (:OnFailure
      (Development|PrintString "Find Session Error"))))

(event EventHandleTravelError
  (params (FailureType :type ETravelFailure%20Enum :default "NoLevel"))
  (Development|PrintString (Utilities|String|EnumtoString FailureType)))