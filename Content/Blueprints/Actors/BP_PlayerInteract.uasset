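; BP_PlayerInteract is a trigger actor that starts a dialogue offering the player a companion-built building.
; Box overlap, gated by a resettable DoOnce, opens the dialogue widget and blends the view to a cinema camera while Tick turns the player toward the companion.
; Cancel restores the player view and re-arms the trigger.
; BeginBuilding also restores it, passing RefBuilding and its build point to the companion's AI controller and switching its behavior.
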(event OnComponentBeginOverlap(Box)
  (params (OverlappedComponent :type Primitive%20Component%20Object%20Reference) (OtherActor :type Actor%20Object%20Reference) (OtherComp :type Primitive%20Component%20Object%20Reference) (OtherBodyIndex :type Integer) (bFromSweep :type Boolean) (SweepResult :type Hit%20Result%20Structure%20%28by%20ref%29))
  (Utilities|FlowControl|DoOnce false
    (:Completed
      (bind _asbp_character_master (Utilities|Casting|CastToBP_Character_Master OtherActor))
      (Variables|Default|SetAs%20BP%20Character%20Master _asbp_character_master)
      (bind _returnvalue (UserInterface|CreateWidget "/Game/Blueprints/Actors/BP_DialogueContruct.BP_DialogueContruct_C" 0 self (Variables|Default|GetDialogue)))
      (UserInterface|Viewport|AddtoViewport _returnvalue 0)
      (CallFunction|ModeCinematic true (Variables|Default|GetCinema%20Camera)))))

(event Custom|Begin%20Building
  (bind _ref_building (Variables|Default|GetRef%20Building))
  (bind _asbp_ai_controller_compagnon (Utilities|Casting|CastToBP_AI_ControllerCompagnon (AI|GetAIController (Variables|/Game/Blueprints/BP_Character_Master.BP_Character_Master_C|GetAs%20BP%20Monster%20Cute (Variables|Default|GetAs%20BP%20Character%20Master)))))
  (AI|SetFocus _asbp_ai_controller_compagnon _ref_building)
  (Default|SetPositionBuilding _asbp_ai_controller_compagnon (Transformation|GetWorldLocation (Variables|/Game/Blueprints/Actors/BP_Construct.BP_Construct_C|GetPointForBuilding _ref_building)) _ref_building)
  (Default|UpdateBehaviorMonsterCute _asbp_ai_controller_compagnon "NewEnumerator1")
  (CallFunction|RotatePlayertoCompagnon)
  (CallFunction|ModeCinematic false (Game|GetPlayerCharacter 0)))

(event Custom|Cancel
  (CallFunction|ModeCinematic false (Game|GetPlayerCharacter 0))
  (Utilities|FlowControl|DoOnce false) ; enters at Reset
)

(event EventTick
  (params (DeltaSeconds :type Float%20%28single-precision%29))
  (CallFunction|RotatePlayertoCompagnon))

(fn ConstructionScript)

(fn RotatePlayertoCompagnon
  (bind _returnvalue (Game|GetPlayerCharacter 0))
  (if (Variables|Default|GetCinematic)
    (bind _as_bp_monster_cute (Variables|/Game/Blueprints/BP_Character_Master.BP_Character_Master_C|GetAs%20BP%20Monster%20Cute (Variables|Default|GetAs%20BP%20Character%20Master))
      (:then
        (Transformation|SetActorRotation _returnvalue (Math|Rotator|MakeRotator 0.0 0.0 (.yaw (Math|Rotator|FindLookatRotation (Transformation|GetActorLocation _returnvalue) (Transformation|GetActorLocation _as_bp_monster_cute)))) true))
      (:else))))

(fn ModeCinematic
  (params (Cinematic :type Boolean) (Target%20Camera :type Actor%20Object%20Reference))
  (bind _returnvalue (Game|GetPlayerController 0))
  (Game|Player|SetViewTargetwithBlend _returnvalue Target%20Camera 1.0 "VTBlend_Linear" 1.0 false)
  (Input|EnableInput (Pawn|GetControlledPawn _returnvalue) _returnvalue)
  (Variables|Default|SetCinematic Cinematic))