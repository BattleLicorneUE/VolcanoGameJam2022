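; BP_Organics_Child is a damageable organic plant actor, derived from a parent Blueprint, that spawns a parasite plant enemy nearby.
; Its Build event runs the parent logic, waits a random delay derived from TimeEventPlantEnnemies, then spawns one BP_Plant_Parasite at a random reachable point around itself and stores the reference.
; Incoming damage reduces PlantHealth, and the actor destroys itself once health is depleted.
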(event EventBeginPlay
  (|CallParentFunction) ; This node is disabled and will not be called.\nDrag off pins to build functionality.
)

(event Collision|EventActorBeginOverlap
  (params (OtherActor :type Actor%20Object%20Reference))
  (|CallParentFunction OtherActor) ; This node is disabled and will not be called.\nDrag off pins to build functionality.
)

(event EventTick
  (params (DeltaSeconds :type Float%20%28single-precision%29))
  (|CallParentFunction DeltaSeconds) ; This node is disabled and will not be called.\nDrag off pins to build functionality.
)

(event EventBuild
  (bind _time_event_plant_ennemies (Variables|Default|GetTime%20Event%20Plant%20Ennemies))
  (|CallParentFunction)
  (Utilities|FlowControl|Delay (Math|Random|RandomFloatinRange _time_event_plant_ennemies (Math|Float|%(Float) _time_event_plant_ennemies 4e+01)))
  (bind _returnvalue (Game|SpawnActorfromClass "/Game/Meshes/Gameplants/BP_Plant_Parasite.BP_Plant_Parasite_C" (Math|Transform|MakeTransform (.RandomLocation (AI|Navigation|GetRandomReachablePointinRadius (Transformation|GetActorLocation) 2e+02 0 0)) "0, 0, 0" "1.000000,1.000000,1.000000") "AlwaysSpawn" 0 0))
  (Variables|Default|SetBP_Plant_Enemies _returnvalue))

(event Game|Damage|EventAnyDamage
  (params (Damage :type Float%20%28single-precision%29) (DamageType :type Damage%20Type%20Object%20Reference) (InstigatedBy :type Controller%20Object%20Reference) (DamageCauser :type Actor%20Object%20Reference))
  (bind _output_get (Variables|Default|SetPlant%20Health (- (Variables|Default|GetPlant%20Health) Damage)))
  (if (<= _output_get 0.0)
    (Actor|DestroyActor)))

(fn ConstructionScript
  (|CallParentFunction))