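; Zone manager actor that tracks a zone's Corrupted, Clean or Complete status and lets the player clean it.
; On overlap it shows status and cleanup-prompt widgets; interacting spends the player's monster calories to set Clean.
; Looping timers run alongside status checks that mark Complete when all valid construct slots are built and swap the floor Niagara effect for corruption.
; The construction script scales components and particle spawn rate from one scale.
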(event OnComponentBeginOverlap(ManagerZone)
  (params (OverlappedComponent :type Primitive%20Component%20Object%20Reference) (OtherActor :type Actor%20Object%20Reference) (OtherComp :type Primitive%20Component%20Object%20Reference) (OtherBodyIndex :type Integer) (bFromSweep :type Boolean) (SweepResult :type Hit%20Result%20Structure%20%28by%20ref%29)))

(event OnComponentEndOverlap(ManagerZone)
  (params (OverlappedComponent :type Primitive%20Component%20Object%20Reference) (OtherActor :type Actor%20Object%20Reference) (OtherComp :type Primitive%20Component%20Object%20Reference) (OtherBodyIndex :type Integer)))

(event Custom|CheckZoneStatus
  (bind _niagara (Variables|Default|GetNiagara))
  (if (Utilities|Enum|Equal(Enum) (Variables|Default|GetZoneStatus) (Utilities|Text|MakeLiteralText "Corrupted"))
    (Class|NiagaraComponent|SetAsset _niagara "/Game/VFX/NS_FloorPourrie.NS_FloorPourrie" true)
    (else
      (Class|NiagaraComponent|SetAsset _niagara "/Game/VFX/NS_FloorSaint.NS_FloorSaint" true))))

(event Custom|CheckCompleteStatus
  (bind _array_element (Utilities|Array|ForEachLoopwithBreak (Variables|Default|GetZoneConstructSlots) :!label _label)
    (:LoopBody
      (Utilities|IsValid _array_element
        (:Is%20Valid
          (if (Variables|/Game/Blueprints/Constructions/BP_Socket.BP_Socket_C|GetFinish%20Build _array_element)
            (Variables|Default|SetZoneComplete? true)
            (else
              (Variables|Default|SetZoneComplete? false)
              (goto _label Break))))))
    (:Completed
      (if (Variables|Default|GetZoneComplete?)
        (Variables|Default|SetZoneStatus "Complete")))))

(event EventBeginPlay
  (Utilities|Time|SetTimerbyEvent (EventDispatchers|CreateEvent :!event Custom|CheckZoneStatus) 0.333333 true)
  (Utilities|Time|SetTimerbyEvent (EventDispatchers|CreateEvent :!event Custom|CheckCompleteStatus) 0.333333 true))

(event Collision|EventActorBeginOverlap
  (params (OtherActor :type Actor%20Object%20Reference)))

(event EventTick
  (params (DeltaSeconds :type Float%20%28single-precision%29)))

(event EventOnInteract
  (bind _asbp_character_master (Utilities|Casting|CastToBP_Character_Master (Game|GetPlayerCharacter 0)))
  (if (>= (Variables|/Game/Blueprints/AI/Compagnon/BP_Compagnon.BP_Compagnon_C|GetCurrentCalorie (Variables|/Game/Blueprints/BP_Character_Master.BP_Character_Master_C|GetAs%20BP%20Monster%20Cute _asbp_character_master)) (Variables|Default|Getcaloriecost))
    (Variables|/Game/Blueprints/AI/Compagnon/BP_Compagnon.BP_Compagnon_C|SetCurrentCalorie (Variables|/Game/Blueprints/BP_Character_Master.BP_Character_Master_C|GetAs%20BP%20Monster%20Cute _asbp_character_master) (- (Variables|/Game/Blueprints/AI/Compagnon/BP_Compagnon.BP_Compagnon_C|GetCurrentCalorie (Variables|/Game/Blueprints/BP_Character_Master.BP_Character_Master_C|GetAs%20BP%20Monster%20Cute _asbp_character_master)) (Variables|Default|Getcaloriecost)))
    (Variables|Default|SetZoneStatus "Clean")))

(event EventOnExitOverlap
  (bind _interactmessage (Variables|Default|GetInteractMessage))
  (Utilities|FlowControl|Sequence
    (:then_0
      (Utilities|IsValid _interactmessage
        (:Is%20Valid
          (Widget|RemovefromParent _interactmessage))))
    (:then_1
      (Widget|RemovefromParent (Variables|Default|GetZoneManageWidget)))))

(event EventOnOverlap
  (bind _zonestatus (Variables|Default|GetZoneStatus))
  (bind _returnvalue (UserInterface|CreateWidget "/Game/Interfaces/RessourceManagement/W_ZoneManagement.W_ZoneManagement_C" 0 (Variables|Default|GetZoneStatus) 0 self))
  (UserInterface|Viewport|AddtoViewport _returnvalue 0)
  (Variables|Default|SetZoneManageWidget _returnvalue)
  (if (not (Utilities|Enum|Equal(Enum) _zonestatus (Utilities|Text|MakeLiteralText "Clean")))
    (if (not (Utilities|Enum|Equal(Enum) _zonestatus (Utilities|Text|MakeLiteralText "Complete")))
      (bind _returnvalue_2 (UserInterface|CreateWidget "/Game/Interfaces/InteractInterfaces/W_InteractMessage.W_InteractMessage_C" 0 (Utilities|Text|FormatText "clean the zone with {value} calories" (Variables|Default|Getcaloriecost))))
      (UserInterface|Viewport|AddtoViewport _returnvalue_2 0)
      (Variables|Default|SetInteractMessage _returnvalue_2))))

(fn ConstructionScript
  (bind _new_scale (Variables|Default|GetNew%20Scale))
  (Transformation|SetWorldScale3D (Variables|Default|GetPlane) _new_scale)
  (Transformation|SetWorldScale3D (Variables|Default|GetManagerZone) (* _new_scale 1.5))
  (Transformation|SetWorldScale3D (Variables|Default|GetStaticMesh) (* _new_scale 0.09))
  (Niagara|SetNiagaraVariable(Float) (Variables|Default|GetNiagara) "SpawnRateParticles" (* (.X (Math|Vector|BreakVector _new_scale)) (Variables|Default|GetParticlesSpawn))))