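; Actor component that gives a character melee weapon equip, unequip and combo attacks against BP_Monster.
; Equip toggle plays montages whose notifies set BEquiped and snap the BP_Character_Master weapon mesh between hand and stowed sockets.
; ATK cycles through a montage array while equipped, with DoOnce gates blocking re-entry.
; Attack notifies fire a forward sphere trace, ignoring owner and its AsBPMonsterCute, to apply point damage, with debug draw and prints.
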(event Custom|ATK
  (if (Variables|Default|GetB_Equiped)
    ;[1 1 1] Play Animation Sword
    (Utilities|FlowControl|DoOnce false :!label _label
      (:Completed
        (bind _notifyname (Animation|Montage|PlayMontage (Variables|/Script/Engine.Character|GetMesh (Variables|Default|GetAs%20Character)) (Utilities|Array|Get(acopy) (Variables|Default|GetMontage%20to%20Play) (Variables|Default|GetIndexATK)) 1.5)
          (:then
            ;[1 1 1] Combot
            (if (<= (Utilities|Array|LastIndex (Variables|Default|GetMontage%20to%20Play)) (Variables|Default|GetIndexATK))
              (Variables|Default|SetIndexATK 0)
              (else
                (Math|Integer|IncrementInt (Variables|Default|GetIndexATK)))))
          (:OnCompleted
            (goto _label Reset))
          (:OnInterrupted
            (Utilities|FlowControl|Delay 1.0)
            (goto _label Reset))
          (:OnNotifyBegin
            (switch name _notifyname
              (:Hit
                (CallFunction|SpawnCollisiontoDamage)))))))))

(event Custom|Spawn%20Collision%20to%20Damage
  (bind _returnvalue (Components|GetOwner))
  (bind _as_character (Variables|Default|GetAs%20Character))
  (bind _returnvalue_2 (Transformation|GetActorLocation _as_character))
  ;[1 1 1] Apply Damages
  (bind _outhit (Collision|SphereTraceForObjects _returnvalue_2 (+ _returnvalue_2 (* (Transformation|GetActorForwardVector _as_character) 2e+02)) 1e+02 (Utilities|Array|MakeArray "ObjectTypeQuery3") false (Utilities|Array|MakeArray _returnvalue (Variables|/Game/Blueprints/BP_Character_Master.BP_Character_Master_C|GetAs%20BP%20Monster%20Cute (.AsBP%20Character%20Master (Utilities|Casting|CastToBP_Character_Master _returnvalue)))) "ForDuration"))
  (bind _asbp_monster (Utilities|Casting|CastToBP_Monster (.HitActor (Collision|BreakHitResult _outhit)))
    (:then
      (bind _returnvalue_3 (Game|Damage|ApplyPointDamage _asbp_monster 5e+01 (.Location (Collision|BreakHitResult _outhit)) _outhit))
      (Development|PrintString (Utilities|String|ToString(Float) _returnvalue_3)))
    (:CastFailed
      (Development|PrintString "Cast Fail hit"))))

(event Custom|Unequiped
  (Utilities|FlowControl|DoOnce false :!label _label
    (:Completed
      (bind _notifyname (Animation|Montage|PlayMontage (Variables|/Script/Engine.Character|GetMesh (Variables|Default|GetAs%20Character)) "/Game/Characters/RetargetingAnimations/EquipedSword/Anim_CS_unEQ1_Montage.Anim_CS_unEQ1_Montage")
        (:OnCompleted
          (goto _label Reset))
        (:OnNotifyBegin
          (switch name _notifyname
            (:Event
              (Variables|Default|SetB_Equiped false)
              (bind _asbp_character_master (Utilities|Casting|CastToBP_Character_Master (Variables|Default|GetAs%20Character)))
              (Transformation|AttachComponentToComponent (Variables|/Game/Blueprints/BP_Character_Master.BP_Character_Master_C|GetStaticMesh _asbp_character_master) (Variables|/Script/Engine.Character|GetMesh _asbp_character_master) "Sword_UnEquiped" "SnapToTarget" "SnapToTarget" "SnapToTarget" true))))))))

(event Custom|Equiped
  (Utilities|FlowControl|DoOnce false :!label _label
    (:Completed
      (bind _notifyname (Animation|Montage|PlayMontage (Variables|/Script/Engine.Character|GetMesh (Variables|Default|GetAs%20Character)) "/Game/Characters/RetargetingAnimations/EquipedSword/Anim_CS_unEQ_to_BOW_EQ1_Montage.Anim_CS_unEQ_to_BOW_EQ1_Montage")
        (:OnCompleted
          (goto _label Reset))
        (:OnNotifyBegin
          (switch name _notifyname
            (:Event
              (Variables|Default|SetB_Equiped true)
              (bind _asbp_character_master (Utilities|Casting|CastToBP_Character_Master (Variables|Default|GetAs%20Character)))
              (Transformation|AttachComponentToComponent (Variables|/Game/Blueprints/BP_Character_Master.BP_Character_Master_C|GetStaticMesh _asbp_character_master) (Variables|/Script/Engine.Character|GetMesh _asbp_character_master) "Weapon" "SnapToTarget" "SnapToTarget" "SnapToTarget" true))))))))

(event Custom|Press%20to%20Equiped/UnEquiped
  (if (Variables|Default|GetB_Equiped)
    (CallFunction|Unequiped)
    (else
      (CallFunction|Equiped))))

(event EventBeginPlay
  (bind _ascharacter (Utilities|Casting|CastToCharacter (Components|GetOwner)))
  (Variables|Default|SetAs%20Character _ascharacter))