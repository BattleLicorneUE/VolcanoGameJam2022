(event OnComponentBeginOverlap(Sphere)
  (params (OverlappedComponent :type Primitive%20Component%20Object%20Reference) (OtherActor :type Actor%20Object%20Reference) (OtherComp :type Primitive%20Component%20Object%20Reference) (OtherBodyIndex :type Integer) (bFromSweep :type Boolean) (SweepResult :type Hit%20Result%20Structure%20%28by%20ref%29))
  (bind _asbp_character_master (Utilities|Casting|CastToBP_Character_Master OtherActor))
  (bind _as_bp_monster_cute (Variables|/Game/Blueprints/BP_Character_Master.BP_Character_Master_C|GetAs%20BP%20Monster%20Cute _asbp_character_master)
    (:then
      (Rendering|SetVisibility (Variables|/Game/Blueprints/AI/Compagnon/BP_Compagnon.BP_Compagnon_C|GetWidget _as_bp_monster_cute) true false)
      (Default|UpdateWidgetDialogue _as_bp_monster_cute (Variables|CustomBuilding|GetDescription%20Building%20by%20Compagnon))
      (Rendering|SetVisibility (Variables|Default|GetWidget) true false)
      (Variables|Other|SetCanInteract true))
    (:else)))

(event OnComponentEndOverlap(Sphere)
  (params (OverlappedComponent :type Primitive%20Component%20Object%20Reference) (OtherActor :type Actor%20Object%20Reference) (OtherComp :type Primitive%20Component%20Object%20Reference) (OtherBodyIndex :type Integer))
  (bind _asbp_character_master (Utilities|Casting|CastToBP_Character_Master OtherActor))
  (bind _as_bp_monster_cute (Variables|/Game/Blueprints/BP_Character_Master.BP_Character_Master_C|GetAs%20BP%20Monster%20Cute _asbp_character_master)
    (:then
      (Rendering|SetVisibility (Variables|/Game/Blueprints/AI/Compagnon/BP_Compagnon.BP_Compagnon_C|GetWidget _as_bp_monster_cute) false false)
      (Default|UpdateWidgetDialogue _as_bp_monster_cute)
      (Rendering|SetVisibility (Variables|Default|GetWidget) false false)
      (Variables|Other|SetCanInteract false))
    (:else)))

(event Custom|Building
  (bind _delay_evolution_random (Variables|CustomBuilding|GetDelay%20Evolution%20Random))
  (bind _origin_vfx (Variables|Default|GetOrigin%20VFX))
  (bind _returnvalue (Transformation|GetWorldLocation _origin_vfx))
  (Utilities|FlowControl|Sequence
    (:then_0
      (Utilities|FlowControl|Delay (Variables|CustomBuilding|GetDelay%20Building%20))
      (Rendering|Material|SetMaterial (Variables|Default|GetPreview) 0 (Variables|CustomBuilding|GetMaterial%20Before%20Building))
      (bind _vfx_finish_building (Variables|CustomBuilding|GetVFX%20Finish%20Building)
        (:then
          (Niagara|SpawnSystematLocation _vfx_finish_building _returnvalue))
        (:else
          _))
      (bind _sound_vfx_finish (Variables|CustomBuilding|GetSound%20VFX%20Finish)
        (:then
          (Audio|PlaySoundatLocation _sound_vfx_finish _returnvalue "0, 0, 0" 1.0 1.0 0.0 0 0 0 0))
        (:else
          _))
      (Variables|Other|SetFinish%20Build true)
      (if (Variables|CustomBuilding|GetEvolution%20)
        (Utilities|FlowControl|Delay (Math|Random|RandomFloatinRange _delay_evolution_random (Math|Float|%(Float) _delay_evolution_random 3e+01)))
        (bind _vfx_finish_building_2 (Variables|CustomBuilding|GetVFX%20Finish%20Building)
          (:then
            (Niagara|SpawnSystematLocation _vfx_finish_building_2 (Transformation|GetWorldLocation (Variables|Default|GetOrigin%20VFX))))
          (:else
            _))
        (Components|StaticMesh|SetStaticMesh (Variables|Default|GetPreview) (Variables|CustomBuilding|GetStatic%20Mesh%20Evolution%20))))
    (:then_1
      (if (Variables|CustomBuilding|GetEvent%20Enable)
        (CallFunction|EventforBuilding)))))

(event Custom|Event%20For%20Building
  (switch Utilities|FlowControl|Switch|SwitchonE_Type_Construction (Variables|CustomBuilding|GetType%20Actor)
    (:NewEnumerator1
      (Utilities|FlowControl|Delay (Math|Random|RandomFloatinRange 15.0 4e+01))
      (Game|SpawnActorfromClass "/Game/Blueprints/AI/BP_Renard/BP_Renard.BP_Renard_C" (Math|Transform|MakeTransform (.RandomLocation (AI|Navigation|GetRandomReachablePointinRadius (Transformation|GetActorLocation) 3e+02 0 0)) "0, 0, 0" "0.300000,0.300000,0.300000") "AlwaysSpawn" 0 0))
    (:NewEnumerator2
      (Utilities|FlowControl|Sequence
        (:then_0
          (Utilities|FlowControl|Delay (Math|Random|RandomFloatinRange 15.0 4e+01))
          (Game|SpawnActorfromClass "/Game/Blueprints/InteractSystem/Int_PetFood.Int_PetFood_C" (Math|Transform|MakeTransform (.RandomLocation (AI|Navigation|GetRandomReachablePointinRadius (Transformation|GetActorLocation) 3e+02 0 0)) "0, 0, 0" "0.300000,0.300000,0.300000") "AlwaysSpawn" 0 0))
        (:then_1
          (Utilities|FlowControl|Delay (Math|Random|RandomFloatinRange 5.0 2e+01) :!label _label)
          (if (Math|Random|RandomBool)
            (Game|SpawnActorfromClass "/Game/Blueprints/Constructions/BP_PlantToxic.BP_PlantToxic_C" (Math|Transform|MakeTransform (.RandomLocation (AI|Navigation|GetRandomReachablePointinRadius (Transformation|GetActorLocation) 3e+02 0 0)) "0, 0, 0" "0.300000,0.300000,0.300000") "AlwaysSpawn" 0 self 0)
            (else
              (goto _label))))))))

(event Custom|Remove%20to%20Interact
  (Variables|/Script/Engine.PrimitiveComponent|SetbGenerateOverlapEvents (Variables|Default|GetSphere) false)
  (bind _asbp_character_master (Utilities|Casting|CastToBP_Character_Master (Game|GetPlayerCharacter 0)))
  (bind _as_bp_monster_cute (Variables|/Game/Blueprints/BP_Character_Master.BP_Character_Master_C|GetAs%20BP%20Monster%20Cute _asbp_character_master)
    (:then
      (Rendering|SetVisibility (Variables|/Game/Blueprints/AI/Compagnon/BP_Compagnon.BP_Compagnon_C|GetWidget _as_bp_monster_cute) false false)
      (Default|UpdateWidgetDialogue _as_bp_monster_cute)
      (Rendering|SetVisibility (Variables|Default|GetWidget) false false)
      (Variables|Other|SetCanInteract false))
    (:else)))

(event EventBeginPlay
  (if (Variables|CustomBuilding|GetAutoConstruct)
    (CallFunction|Building)))

(event EventUpdateImpact
  (switch Utilities|FlowControl|Switch|SwitchonE_Type_Construction (Variables|CustomBuilding|GetType%20Actor)
    (:NewEnumerator0
      (if (Variables|Other|GetFinish%20Build)
        (bind _asbp_character_master (Utilities|Casting|CastToBP_Character_Master (Game|GetPlayerCharacter 0)))
        (Default|AddCarbonValue _asbp_character_master (Variables|Default|GetAdd%20Carbon%20Value%20))
        (Default|RemoveAirValue _asbp_character_master (Variables|Default|GetRemove%20air%20value))))
    (:NewEnumerator2
      (if (Variables|Other|GetFinish%20Build)
        (bind _asbp_character_master_2 (Utilities|Casting|CastToBP_Character_Master (Game|GetPlayerCharacter 0)))
        (Default|AddAirValue _asbp_character_master_2 (Variables|Default|GetAdd%20Air%20Value))
        (Default|RemoveCarbonValue _asbp_character_master_2 (Variables|Default|GetRemove%20Carbon%20Value))))))

(event Game|Damage|EventAnyDamage
  (params (Damage :type Float%20%28single-precision%29) (DamageType :type Damage%20Type%20Object%20Reference) (InstigatedBy :type Controller%20Object%20Reference) (DamageCauser :type Actor%20Object%20Reference))
  (bind _output_get (Variables|CustomBuilding|SetHealth (Math|Float|Clamp(Float) (- (Variables|CustomBuilding|GetHealth) Damage) 0.0 (Variables|CustomBuilding|GetHealth))))
  (if (<= _output_get 0.0)
    (bind _vfx_building_destoyer (Variables|CustomBuilding|GetVFX%20Building%20Destoyer)
      (:then
        (Niagara|SpawnSystematLocation _vfx_building_destoyer (Transformation|GetWorldLocation (Variables|Default|GetOrigin%20VFX))))
      (:else
        _))
    (bind _sound_destroyer (Variables|CustomBuilding|GetSound%20Destroyer)
      (:then
        (Audio|PlaySoundatLocation _sound_destroyer "0, 0, 0" "0, 0, 0" 1.0 1.0 0.0 0 0 0 0))
      (:else
        _))
    (Actor|DestroyActor)))

(event Input|KeyboardEvents|E
  (params (Key :type Key%20Structure :default "None"))
  (:Pressed
    (if (Variables|Other|GetCanInteract)
      (CallFunction|Building)
      (CallFunction|RemovetoInteract))))

(fn ConstructionScript
  (bind _preview (Variables|Default|GetPreview))
  (Components|StaticMesh|SetStaticMesh _preview (Variables|CustomEditor|GetStatic%20Preview))
  (Rendering|Material|SetMaterial _preview 0 (Variables|CustomEditor|GetMaterial%20Preview%20Mesh)))